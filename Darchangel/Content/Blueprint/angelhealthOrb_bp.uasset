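; Angel health orb pickup that homes in on the player's demonicForm_bp character and restores its AngelHealth.
; Each tick, while that health is below 100, it interpolates its location toward the player pawn.
; On box overlap with that character below 100, it adds a fixed amount, calls AngelHeal and destroys itself.
; It also self-destructs a few seconds after BeginPlay if not collected.
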(event OnComponentBeginOverlap(Box)
  (params (OverlappedComponent :type Primitive%20Component%20Object%20Reference) (OtherActor :type Actor%20Object%20Reference) (OtherComp :type Primitive%20Component%20Object%20Reference) (OtherBodyIndex :type Integer) (bFromSweep :type Boolean) (SweepResult :type Hit%20Result%20Structure%20%28by%20ref%29))
  (bind _asdemonic_form_bp (Utilities|Casting|CastTodemonicForm_bp OtherActor))
  (if (not (>= (Variables|/Game/Blueprint/demonicForm_bp.demonicForm_bp_C|GetangelHealth _asdemonic_form_bp) 1e+02))
    (Variables|/Game/Blueprint/demonicForm_bp.demonicForm_bp_C|SetangelHealth _asdemonic_form_bp (+ (Variables|/Game/Blueprint/demonicForm_bp.demonicForm_bp_C|GetangelHealth _asdemonic_form_bp) 3e+01))
    (Default|AngelHeal _asdemonic_form_bp)
    (Actor|DestroyActor)))

(event EventBeginPlay
  (Utilities|FlowControl|Delay 3.0)
  (Actor|DestroyActor))

(event Collision|EventActorBeginOverlap
  (params (OtherActor :type Actor%20Object%20Reference)))

(event EventTick
  (params (DeltaSeconds :type Float%20%28single-precision%29))
  (bind _returnvalue (Game|Player|GetPlayerPawn 0))
  (bind _asdemonic_form_bp (Utilities|Casting|CastTodemonicForm_bp (Game|GetPlayerCharacter 0)))
  (if (not (>= (Variables|/Game/Blueprint/demonicForm_bp.demonicForm_bp_C|GetangelHealth _asdemonic_form_bp) 1e+02))
    (Transformation|SetActorLocation (Math|Interpolation|VInterpTo (Transformation|GetActorLocation) (+ (Transformation|GetActorLocation _returnvalue) (* (Transformation|GetActorForwardVector _returnvalue) 0.0)) DeltaSeconds 3.0) false false)))

(fn ConstructionScript)