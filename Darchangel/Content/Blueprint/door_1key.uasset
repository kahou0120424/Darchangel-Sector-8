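; A double door that swings open when a demonicForm_bp character carrying at least RequiredKeys overlaps its collision.
; With too few keys, the character's interact indicator shows instead and hides again when the overlap ends.
; Two timelines lerp the right and left door rotations to their target rotators, with no closing logic.
; Key deduction and key-indicator widget creation are unconnected, so keys are not consumed.
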(event OnComponentBeginOverlap(DoorCollision)
  (params (OverlappedComponent :type Primitive%20Component%20Object%20Reference) (OtherActor :type Actor%20Object%20Reference) (OtherComp :type Primitive%20Component%20Object%20Reference) (OtherBodyIndex :type Integer) (bFromSweep :type Boolean) (SweepResult :type Hit%20Result%20Structure%20%28by%20ref%29))
  (Variables|Default|SetisPressed true)
  (bind _asdemonic_form_bp (Utilities|Casting|CastTodemonicForm_bp OtherActor))
  (Utilities|FlowControl|Sequence
    (:then_0
      (if (< (Variables|/Game/Blueprint/demonicForm_bp.demonicForm_bp_C|GetnumberofKeys _asdemonic_form_bp) (Variables|Default|GetrequiredKeys))
        (Utilities|FlowControl|Sequence
          (:then_0
            (Rendering|SetVisibility (Variables|/Game/Blueprint/demonicForm_bp.demonicForm_bp_C|GetInteractIndicator _asdemonic_form_bp) true false)))
        (else
          (Rendering|SetVisibility (Variables|/Game/Blueprint/demonicForm_bp.demonicForm_bp_C|GetInteractIndicator _asdemonic_form_bp) false false))))
    (:then_1
      (if (>= (Variables|/Game/Blueprint/demonicForm_bp.demonicForm_bp_C|GetnumberofKeys _asdemonic_form_bp) (Variables|Default|GetrequiredKeys))
        (Utilities|FlowControl|Sequence
          (:then_0
            (bind _alpha (Timeline|RightDoorMovement Play)
              (:Update
                (Transformation|SetRelativeRotation (Variables|Default|GetRightDoor) (Math|Rotator|Lerp(Rotator) "0,0.000000, 0" (Variables|Default|GetrightLocation) _alpha) false false))))
          (:then_1
            (bind _alpha_2 (Timeline|LeftDoorMovement Play)
              (:Update
                (Transformation|SetRelativeRotation (Variables|Default|GetLeftDoor) (Math|Rotator|Lerp(Rotator) "0,180.000000,0.000000" (Variables|Default|GetleftLocation) _alpha_2) false false)))))))))

(event OnComponentEndOverlap(DoorCollision)
  (params (OverlappedComponent :type Primitive%20Component%20Object%20Reference) (OtherActor :type Actor%20Object%20Reference) (OtherComp :type Primitive%20Component%20Object%20Reference) (OtherBodyIndex :type Integer))
  (Variables|Default|SetisPressed false)
  (bind _asdemonic_form_bp (Utilities|Casting|CastTodemonicForm_bp OtherActor))
  (Utilities|FlowControl|Sequence
    (:then_0
      (Utilities|FlowControl|Delay 3.0))
    (:then_1
      (Rendering|SetVisibility (Variables|/Game/Blueprint/demonicForm_bp.demonicForm_bp_C|GetInteractIndicator _asdemonic_form_bp) false false))))

(event EventBeginPlay)

(event Collision|EventActorBeginOverlap
  (params (OtherActor :type Actor%20Object%20Reference)))

(event EventTick
  (params (DeltaSeconds :type Float%20%28single-precision%29)))

(fn ConstructionScript)