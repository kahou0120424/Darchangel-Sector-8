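; Checkpoint actor that saves or clears the player's respawn data when anything overlaps its Box trigger.
; With its Load flag set, it stores the demonicForm_bp player's location and a Load flag in the SaveTut save game in slot "save1", creating the save if none exists.
; With the flag off, it sets the existing save's Load to false, acting as a checkpoint clearer.
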(event OnComponentBeginOverlap(Box)
  (params (OverlappedComponent :type Primitive%20Component%20Object%20Reference) (OtherActor :type Actor%20Object%20Reference) (OtherComp :type Primitive%20Component%20Object%20Reference) (OtherBodyIndex :type Integer) (bFromSweep :type Boolean) (SweepResult :type Hit%20Result%20Structure%20%28by%20ref%29))
  (if (Variables|Default|GetLoad?)
    (Utilities|FlowControl|Sequence
      (:then_0
        (bind _asdemonic_form_bp (Utilities|Casting|CastTodemonicForm_bp (Game|GetPlayerCharacter 0)))
        (Variables|Default|SetPlayerLoc (Transformation|GetActorLocation _asdemonic_form_bp))
        (Development|PrintString "Checkpoint Reached!"))
      (:then_1
        (bind _returnvalue (SaveGame|DoesSaveGameExist "save1"))
        (if _returnvalue
          (bind _returnvalue_2 (SaveGame|LoadGamefromSlot "save1"))
          (bind _assave_tut (Utilities|Casting|CastToSaveTut _returnvalue_2))
          (Variables|/Game/Blueprint/Checkpoint/SaveTut.SaveTut_C|SetPlayerLoc.s _assave_tut (Variables|Default|GetPlayerLoc))
          (Variables|/Game/Blueprint/Checkpoint/SaveTut.SaveTut_C|SetLoad? _assave_tut true)
          (SaveGame|SaveGametoSlot _assave_tut "save1")
          (else
            (bind _returnvalue_3 (SaveGame|CreateSaveGameObject "/Game/Blueprint/Checkpoint/SaveTut.SaveTut_C"))
            (Variables|/Game/Blueprint/Checkpoint/SaveTut.SaveTut_C|SetPlayerLoc.s _returnvalue_3 (Variables|Default|GetPlayerLoc))
            (Variables|/Game/Blueprint/Checkpoint/SaveTut.SaveTut_C|SetLoad? _returnvalue_3 true)
            (SaveGame|SaveGametoSlot _returnvalue_3 "save1")
            (Development|PrintString "Checkpoint Reached")))))
    (else
      (bind _returnvalue_4 (SaveGame|LoadGamefromSlot "save1"))
      (bind _assave_tut_2 (Utilities|Casting|CastToSaveTut _returnvalue_4))
      (Variables|/Game/Blueprint/Checkpoint/SaveTut.SaveTut_C|SetLoad? _assave_tut_2 false)
      (SaveGame|SaveGametoSlot _assave_tut_2 "save1")
      (Development|PrintString "Checkpoint Cleared"))))

(event EventBeginPlay)

(event Collision|EventActorBeginOverlap
  (params (OtherActor :type Actor%20Object%20Reference)))

(event EventTick
  (params (DeltaSeconds :type Float%20%28single-precision%29)))

(fn ConstructionScript)