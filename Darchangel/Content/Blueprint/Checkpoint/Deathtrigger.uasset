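; Death trigger volume that sends the player's demonicForm_bp character back to the last checkpoint save.
; Any overlap with its Box disables player input, waits briefly, then checks for the "save1" slot, without checking which actor overlapped.
; An existing SaveTut save moves the character to its stored PlayerLoc and restores input; with no save, it opens the Tutorialv3 level.
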(event OnComponentBeginOverlap(Box)
  (params (OverlappedComponent :type Primitive%20Component%20Object%20Reference) (OtherActor :type Actor%20Object%20Reference) (OtherComp :type Primitive%20Component%20Object%20Reference) (OtherBodyIndex :type Integer) (bFromSweep :type Boolean) (SweepResult :type Hit%20Result%20Structure%20%28by%20ref%29))
  (bind _asdemonic_form_bp (Utilities|Casting|CastTodemonicForm_bp (Game|GetPlayerCharacter 0)))
  (Input|DisableInput _asdemonic_form_bp (Game|GetPlayerController 0))
  (Utilities|FlowControl|Delay 0.25)
  (bind _returnvalue (SaveGame|DoesSaveGameExist "save1"))
  (if _returnvalue
    (bind _returnvalue_2 (SaveGame|LoadGamefromSlot "save1"))
    (bind _assave_tut (Utilities|Casting|CastToSaveTut _returnvalue_2))
    (bind _asdemonic_form_bp_2 (Utilities|Casting|CastTodemonicForm_bp (Game|GetPlayerCharacter 0)))
    (Transformation|SetActorLocation _asdemonic_form_bp_2 (Variables|/Game/Blueprint/Checkpoint/SaveTut.SaveTut_C|GetPlayerLoc.s _assave_tut) false false)
    (Input|EnableInput _asdemonic_form_bp_2 (Game|GetPlayerController 0))
    (else
      (Game|OpenLevel(byName) (Variables|Default|GetTutorialv3)))))

(event EventBeginPlay)

(event Collision|EventActorBeginOverlap
  (params (OtherActor :type Actor%20Object%20Reference)))

(event EventTick
  (params (DeltaSeconds :type Float%20%28single-precision%29)))

(fn ConstructionScript)