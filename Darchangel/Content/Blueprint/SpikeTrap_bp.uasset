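; Spike trap actor that damages the player's demon or angel form on overlap and cycles its spike up and down.
; TrapDetect overlap casts to demonicForm_bp and subtracts fixed damage from DemonHealth or AngelHealth, depending on IsDemonForm.
; The SpikeOn timeline lerps the Spike's relative Z position, played by SpikeActivate and reversed by SpikeReset.
; Tick drives both events through Delays inside a loop over all SpikeTrap_bp actors.
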(event OnComponentBeginOverlap(TrapDetect)
  (params (OverlappedComponent :type Primitive%20Component%20Object%20Reference) (OtherActor :type Actor%20Object%20Reference) (OtherComp :type Primitive%20Component%20Object%20Reference) (OtherBodyIndex :type Integer) (bFromSweep :type Boolean) (SweepResult :type Hit%20Result%20Structure%20%28by%20ref%29))
  (bind _asdemonic_form_bp (Utilities|Casting|CastTodemonicForm_bp OtherActor))
  (if (Variables|/Game/Blueprint/demonicForm_bp.demonicForm_bp_C|GetisDemonForm _asdemonic_form_bp)
    (Variables|/Game/Blueprint/demonicForm_bp.demonicForm_bp_C|SetdemonHealth _asdemonic_form_bp (- (Variables|/Game/Blueprint/demonicForm_bp.demonicForm_bp_C|GetdemonHealth _asdemonic_form_bp) 5.0))
    (else
      (Variables|/Game/Blueprint/demonicForm_bp.demonicForm_bp_C|SetangelHealth _asdemonic_form_bp (- (Variables|/Game/Blueprint/demonicForm_bp.demonicForm_bp_C|GetangelHealth _asdemonic_form_bp) 5.0)))))

(event Custom|SpikeActivate
  (bind _spikeup (Timeline|SpikeOn Play)
    (:Update
      (Transformation|SetRelativeLocation (Variables|Default|GetSpike) (Math|Vector|Lerp(Vector) "0, 0, 0" "0.000000,0.000000,-350.000000" _spikeup) false false))))

(event Custom|SpikeReset
  (bind _spikeup (Timeline|SpikeOn Reverse)
    (:Update
      (Transformation|SetRelativeLocation (Variables|Default|GetSpike) (Math|Vector|Lerp(Vector) "0, 0, 0" "0.000000,0.000000,-350.000000" _spikeup) false false))))

(event EventBeginPlay)

(event Collision|EventActorBeginOverlap
  (params (OtherActor :type Actor%20Object%20Reference)))

(event EventTick
  (params (DeltaSeconds :type Float%20%28single-precision%29))
  (bind _outactors (Actor|GetAllActorsOfClass "SpikeTrap_bp_C"))
  (for _array_element _outactors
    (Utilities|FlowControl|Delay 8.0)
    (CallFunction|SpikeActivate)
    (Utilities|FlowControl|Delay 9.0)
    (CallFunction|SpikeReset)))

(fn ConstructionScript)