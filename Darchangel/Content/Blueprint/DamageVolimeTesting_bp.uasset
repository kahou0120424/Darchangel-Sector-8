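; Test damage volume that drains the player's demon or angel health while the demonicForm_bp character stands inside its Box.
; Box begin and end overlaps with that character toggle an IsInVolume flag.
; Tick prints the in/out state for debugging and uses a short Delay to throttle damage, subtracting a fixed amount from DemonHealth or AngelHealth according to the player character's IsDemonForm.
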(event OnComponentBeginOverlap(Box)
  (params (OverlappedComponent :type Primitive%20Component%20Object%20Reference) (OtherActor :type Actor%20Object%20Reference) (OtherComp :type Primitive%20Component%20Object%20Reference) (OtherBodyIndex :type Integer) (bFromSweep :type Boolean) (SweepResult :type Hit%20Result%20Structure%20%28by%20ref%29))
  (Utilities|Casting|CastTodemonicForm_bp OtherActor)
  (Variables|Default|SetisInVolume true))

(event OnComponentEndOverlap(Box)
  (params (OverlappedComponent :type Primitive%20Component%20Object%20Reference) (OtherActor :type Actor%20Object%20Reference) (OtherComp :type Primitive%20Component%20Object%20Reference) (OtherBodyIndex :type Integer))
  (Utilities|Casting|CastTodemonicForm_bp OtherActor)
  (Variables|Default|SetisInVolume false))

(event Custom|CustomEvent
  (params (OverlappedComponent :type Primitive%20Component%20Object%20Reference) (OtherActor :type Actor%20Object%20Reference) (OtherComp :type Primitive%20Component%20Object%20Reference) (OtherBodyIndex :type Integer)))

(event EventBeginPlay)

(event Collision|EventActorBeginOverlap
  (params (OtherActor :type Actor%20Object%20Reference)))

(event EventTick
  (params (DeltaSeconds :type Float%20%28single-precision%29))
  (bind _returnvalue (Game|GetPlayerCharacter 0))
  (Utilities|FlowControl|Sequence
    (:then_0
      (if (Variables|Default|GetisInVolume)
        (Development|PrintString "damaging" true true "(R=0.000000,G=0.660000,B=1.000000,A=1.000000)" 0.0)
        (else
          (Development|PrintString "go out" true true "(R=0.000000,G=0.660000,B=1.000000,A=1.000000)" 0.0))))
    (:then_1
      (Utilities|FlowControl|Delay 0.2)
      (if (Variables|Default|GetisInVolume)
        (bind _asdemonic_form_bp (Utilities|Casting|CastTodemonicForm_bp _returnvalue))
        (if (Variables|/Game/Blueprint/demonicForm_bp.demonicForm_bp_C|GetisDemonForm _asdemonic_form_bp)
          (bind _asdemonic_form_bp_2 (Utilities|Casting|CastTodemonicForm_bp _returnvalue))
          (Variables|/Game/Blueprint/demonicForm_bp.demonicForm_bp_C|SetdemonHealth _asdemonic_form_bp_2 (- (Variables|/Game/Blueprint/demonicForm_bp.demonicForm_bp_C|GetdemonHealth _asdemonic_form_bp_2) 1e+01))
          (else
            (bind _asdemonic_form_bp_3 (Utilities|Casting|CastTodemonicForm_bp _returnvalue))
            (Variables|/Game/Blueprint/demonicForm_bp.demonicForm_bp_C|SetangelHealth _asdemonic_form_bp_3 (- (Variables|/Game/Blueprint/demonicForm_bp.demonicForm_bp_C|GetangelHealth _asdemonic_form_bp_3) 1e+01))))))))

(fn ConstructionScript)