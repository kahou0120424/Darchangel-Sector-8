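; Player character Blueprint with a minimap widget, visible mouse cursor and key-triggered abilities.
; T spawns a short-lived Wall of Light at the cursor trace hit, while F and G spawn placeholder Blessed Idol and Grasp of Death actors at component transforms.
; H calls CallSpawnEcho; Tab's form swap only wires one FlipFlop branch, setting the mannequin mesh.
; Capsule overlap with "walloflight"-tagged actors attaches a shield particle above the mesh.
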(event OnComponentBeginOverlap(CapsuleComponent)
  (params (OverlappedComponent :type Primitive%20Component%20Object%20Reference) (OtherActor :type Actor%20Object%20Reference) (OtherComp :type Primitive%20Component%20Object%20Reference) (OtherBodyIndex :type Integer) (bFromSweep :type Boolean) (SweepResult :type Hit%20Result%20Structure%20%28by%20ref%29))
  (bind _mesh (Variables|Character|GetMesh))
  (bind _relativelocation (Variables|/Script/Engine.SceneComponent|GetRelativeLocation _mesh))
  (bind (_x _y _z) (Math|Vector|BreakVector _relativelocation))
  ;[1 1 1] barr
  (if (Actor|ActorHasTag OtherActor "walloflight")
    (Effects|SpawnEmitterAttached "/Game/Shield/shieldParticle.shieldParticle" _mesh "None" (Math|Vector|MakeVector _x _y (+ _z 205.0)))))

(event EventBeginPlay
  (bind _returnvalue (Game|GetPlayerController 0))
  ;[1 1 1] Minimap
  (bind _returnvalue_2 (Game|ConstructObjectfromClass "/Game/Blueprint/MinimapUI/Minimap_Widget.Minimap_Widget_C" _returnvalue))
  (bind _output_get (Variables|Default|SetMinimapWidget _returnvalue_2))
  (UserInterface|Viewport|AddtoViewport _output_get 0)
  ;;[1 1 1] Ingame Cursor
  (Variables|/Script/Engine.PlayerController|SetbShowMouseCursor _returnvalue true))

(event Collision|EventActorBeginOverlap
  (params (OtherActor :type Actor%20Object%20Reference)))

(event EventTick
  (params (DeltaSeconds :type Float%20%28single-precision%29)))

(event Input|KeyboardEvents|Tab
  (params (Key :type Key%20Structure :default "None"))
  ;[1 1 1] Swap Forms
  (:Pressed
    (Utilities|FlowControl|FlipFlop
      (:A
        (Class|SkinnedMeshComponent|SetSkeletalMesh (Variables|Character|GetMesh) "/Game/Mannequin/Character/Mesh/SK_Mannequin.SK_Mannequin" true)))))

(event Input|KeyboardEvents|F
  (params (Key :type Key%20Structure :default "None"))
  (:Pressed
    (Game|SpawnActorfromClass "/Game/ThirdPersonBP/Blueprints/BlessedIdol_PH.BlessedIdol_PH_C" (Transformation|GetWorldTransform (Variables|Default|GetBlessedIdol_Spawn)) "Undefined" 0 0)))

(event Input|KeyboardEvents|G
  (params (Key :type Key%20Structure :default "None"))
  (:Pressed
    (Game|SpawnActorfromClass "/Game/ThirdPersonBP/Blueprints/GraspOfDeath_PH.GraspOfDeath_PH_C" (Transformation|GetWorldTransform (Variables|Default|GetGraspOfDeath_Spawn)) "Undefined" 0 0)))

(event Input|KeyboardEvents|T
  (params (Key :type Key%20Structure :default "None"))
  ;[1 1 1] Wall of Light
  (:Pressed
    (bind _returnvalue (Game|SpawnActorfromClass "/Game/Blueprint/wallSpawned_bp.wallSpawned_bp_C" (Math|Transform|MakeTransform (.Location (Collision|BreakHitResult (.HitResult (Game|Player|GetHitResultUnderCursorbyChannel (Game|GetPlayerController 0) "TraceTypeQuery1" true)))) (Transformation|GetActorRotation (Game|Player|GetPlayerPawn 0))) "Undefined" 0 0))
    (Actor|SetLifeSpan _returnvalue 3.0)))

(event Input|KeyboardEvents|H
  (params (Key :type Key%20Structure :default "None"))
  (:Pressed
    (Default|CallSpawnEcho)))

(fn ConstructionScript)