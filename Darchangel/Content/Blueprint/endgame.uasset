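; Endgame trigger actor that ends the game when the demonic form character overlaps its collision component.
; On overlap it clears all widgets, disables the character's input, plays the end level sequence and teleports the character to a Teleport reference's location.
; After a fixed delay it opens the main menu level.
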(event OnComponentBeginOverlap(CollisionComponent)
  (params (OverlappedComponent :type Primitive%20Component%20Object%20Reference) (OtherActor :type Actor%20Object%20Reference) (OtherComp :type Primitive%20Component%20Object%20Reference) (OtherBodyIndex :type Integer) (bFromSweep :type Boolean) (SweepResult :type Hit%20Result%20Structure%20%28by%20ref%29))
  (bind _asdemonic_form_bp (Utilities|Casting|CastTodemonicForm_bp OtherActor))
  (Viewport|RemoveAllWidgets)
  (Input|DisableInput _asdemonic_form_bp 0)
  (bind _returnvalue (Sequencer|Player|CreateLevelSequencePlayer "/Game/Sequence/endsequence.endsequence"))
  (Sequencer|Player|Play _returnvalue :!class /Script/MovieScene.MovieSceneSequencePlayer)
  (Transformation|Teleport _asdemonic_form_bp (Transformation|GetActorLocation (Variables|Default|Getteleport)) "0, 0, 0")
  (Utilities|FlowControl|Delay 6.0)
  (Game|OpenLevel(byName) "Mainmenu_level"))

(event EventBeginPlay)

(event Collision|EventActorBeginOverlap
  (params (OtherActor :type Actor%20Object%20Reference)))

(event EventTick
  (params (DeltaSeconds :type Float%20%28single-precision%29)))

(fn ConstructionScript)