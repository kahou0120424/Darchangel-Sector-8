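; End-of-game trigger actor that shows closing dialogue and then quits the game.
; Entering its box shows a text prompt, enables the actor's input and halts the demonicForm_bp character; leaving reverses prompt and input.
; TriggerDia removes an existing dialogue widget, or creates one with TriggerText and freezes the player.
; Chained delays then bring up EndGameWidget over it before quitting.
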(event OnComponentBeginOverlap(Box)
  (params (OverlappedComponent :type Primitive%20Component%20Object%20Reference) (OtherActor :type Actor%20Object%20Reference) (OtherComp :type Primitive%20Component%20Object%20Reference) (OtherBodyIndex :type Integer) (bFromSweep :type Boolean) (SweepResult :type Hit%20Result%20Structure%20%28by%20ref%29))
  (Rendering|SetVisibility (Variables|Default|GetTextRender) true false)
  (Input|EnableInput (Game|GetPlayerController 0))
  (bind _asdemonic_form_bp (Utilities|Casting|CastTodemonicForm_bp OtherActor))
  (Components|Movement|StopMovementImmediately (Variables|/Script/Engine.Character|GetCharacterMovement _asdemonic_form_bp)))

(event OnComponentEndOverlap(Box)
  (params (OverlappedComponent :type Primitive%20Component%20Object%20Reference) (OtherActor :type Actor%20Object%20Reference) (OtherComp :type Primitive%20Component%20Object%20Reference) (OtherBodyIndex :type Integer))
  (Rendering|SetVisibility (Variables|Default|GetTextRender) false false)
  (Input|DisableInput (Game|GetPlayerController 0))
  (if (Variables|Default|GetisTriggered)
    (Utilities|FlowControl|Delay 0.5)
    (Widget|RemovefromParent (Variables|Default|GetDialogue%20Widget_end))))

(event EventBeginPlay)

(event Collision|EventActorBeginOverlap
  (params (OtherActor :type Actor%20Object%20Reference)))

(event EventTick
  (params (DeltaSeconds :type Float%20%28single-precision%29)))

(event EventTriggerDia
  (bind _returnvalue (Game|GetPlayerCharacter 0))
  (Utilities|IsValid (Variables|Default|GetDialogue%20Widget_end)
    (:Is%20Valid
      (Widget|RemovefromParent (Variables|Default|GetDialogue%20Widget_end)))
    (:Is%20Not%20Valid
      (bind _returnvalue_2 (UserInterface|CreateWidget "/Game/Blueprint/DialogueSystem/End/Trigger_end.Trigger_end_C" (Game|GetPlayerController 0)))
      (bind _output_get (Variables|Default|SetDialogue%20Widget_end _returnvalue_2))
      (UserInterface|Viewport|AddtoViewport _output_get 0)
      ;[1 1 1] Prob 1 - Cant take Dialogue widget out and edit text
      (Variables|/Game/Blueprint/DialogueSystem/End/Trigger_end.Trigger_end_C|SetdialogueEndText (Variables|Default|GetDialogue%20Widget_end) (Variables|Default|GetTriggerText))
      (bind _asdemonic_form_bp (Utilities|Casting|CastTodemonicForm_bp _returnvalue))
      (Components|Movement|StopMovementImmediately (Variables|/Script/Engine.Character|GetCharacterMovement _asdemonic_form_bp))
      (Input|DisableInput _returnvalue 0)
      (Utilities|FlowControl|Delay 2.0)
      (Utilities|FlowControl|Delay 2.0)
      (bind _returnvalue_3 (UserInterface|CreateWidget "/Game/Blueprint/DialogueSystem/End/EndGameWidget.EndGameWidget_C" (Game|GetPlayerController 0)))
      (UserInterface|Viewport|AddtoViewport _returnvalue_3 2)
      (Utilities|FlowControl|Delay 6.0)
      (Game|QuitGame 0 "Quit" false))))

(fn ConstructionScript)