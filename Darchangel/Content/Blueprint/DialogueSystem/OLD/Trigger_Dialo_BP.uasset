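; Dialogue trigger actor that shows a text prompt when the demonicForm_bp character is near.
; Box overlap toggles that character's InteractIndicator and enables or disables the actor's input for player 0.
; TriggerDia toggles a Trigger_Dialo widget, filling it with TriggerText on creation and setting IsTriggered.
; Leaving the box does not close the widget: the IsTriggered branch is empty and the delayed removal is disconnected.
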(event OnComponentBeginOverlap(Box)
  (params (OverlappedComponent :type Primitive%20Component%20Object%20Reference) (OtherActor :type Actor%20Object%20Reference) (OtherComp :type Primitive%20Component%20Object%20Reference) (OtherBodyIndex :type Integer) (bFromSweep :type Boolean) (SweepResult :type Hit%20Result%20Structure%20%28by%20ref%29))
  (bind _asdemonic_form_bp (Utilities|Casting|CastTodemonicForm_bp OtherActor))
  (Rendering|SetVisibility (Variables|/Game/Blueprint/demonicForm_bp.demonicForm_bp_C|GetInteractIndicator _asdemonic_form_bp) true false)
  (Input|EnableInput (Game|GetPlayerController 0)))

(event OnComponentEndOverlap(Box)
  (params (OverlappedComponent :type Primitive%20Component%20Object%20Reference) (OtherActor :type Actor%20Object%20Reference) (OtherComp :type Primitive%20Component%20Object%20Reference) (OtherBodyIndex :type Integer))
  (bind _asdemonic_form_bp (Utilities|Casting|CastTodemonicForm_bp OtherActor))
  (Rendering|SetVisibility (Variables|/Game/Blueprint/demonicForm_bp.demonicForm_bp_C|GetInteractIndicator _asdemonic_form_bp) false false)
  (Input|DisableInput (Game|GetPlayerController 0))
  (if (Variables|Default|GetisTriggered)
    _))

(event EventBeginPlay)

(event Collision|EventActorBeginOverlap
  (params (OtherActor :type Actor%20Object%20Reference)))

(event EventTick
  (params (DeltaSeconds :type Float%20%28single-precision%29)))

(event EventTriggerDia
  (Utilities|IsValid (Variables|Default|GetDialogueWidget)
    (:Is%20Valid
      (Widget|RemovefromParent (Variables|Default|GetDialogueWidget))
      (Variables|Default|SetDialogueWidget 0))
    (:Is%20Not%20Valid
      (bind _returnvalue (UserInterface|CreateWidget "/Game/Blueprint/DialogueSystem/OLD/Trigger_Dialo.Trigger_Dialo_C" (Game|GetPlayerController 0)))
      (bind _output_get (Variables|Default|SetDialogueWidget _returnvalue))
      (UserInterface|Viewport|AddtoViewport _output_get 0)
      (Variables|/Game/Blueprint/DialogueSystem/OLD/Trigger_Dialo.Trigger_Dialo_C|SetdialogueText (Variables|Default|GetDialogueWidget) (Variables|Default|GetTriggerText))
      (Variables|Default|SetisTriggered true))))

(fn ConstructionScript)