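; Dialogue trigger actor that shows a prompt and an end-dialogue widget for a volume in the level.
; Entering the box reveals its TextRender and enables input, then stops movement if the actor is demonicForm_bp.
; TriggerDia toggles the Trigger_end widget, filling it with TriggerText.
; Exiting hides the prompt and disables input; delayed widget removal depends on IsTriggered, whose only setter is unconnected.
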(event OnComponentBeginOverlap(Box)
  (params (OverlappedComponent :type Primitive%20Component%20Object%20Reference) (OtherActor :type Actor%20Object%20Reference) (OtherComp :type Primitive%20Component%20Object%20Reference) (OtherBodyIndex :type Integer) (bFromSweep :type Boolean) (SweepResult :type Hit%20Result%20Structure%20%28by%20ref%29))
  (Rendering|SetVisibility (Variables|Default|GetTextRender) true false)
  (Input|EnableInput (Game|GetPlayerController 0))
  (bind _asdemonic_form_bp (Utilities|Casting|CastTodemonicForm_bp OtherActor))
  (Components|Movement|StopMovementImmediately (Variables|/Script/Engine.Character|GetCharacterMovement _asdemonic_form_bp)))

(event OnComponentEndOverlap(Box)
  (params (OverlappedComponent :type Primitive%20Component%20Object%20Reference) (OtherActor :type Actor%20Object%20Reference) (OtherComp :type Primitive%20Component%20Object%20Reference) (OtherBodyIndex :type Integer))
  (Rendering|SetVisibility (Variables|Default|GetTextRender) false false)
  (Input|DisableInput (Game|GetPlayerController 0))
  (if (Variables|Default|GetisTriggered)
    (Utilities|FlowControl|Delay 0.5)
    (Widget|RemovefromParent (Variables|Default|GetDialogue%20Widget_end))))

(event EventBeginPlay)

(event Collision|EventActorBeginOverlap
  (params (OtherActor :type Actor%20Object%20Reference)))

(event EventTick
  (params (DeltaSeconds :type Float%20%28single-precision%29)))

(event EventTriggerDia
  (Utilities|IsValid (Variables|Default|GetDialogue%20Widget_end)
    (:Is%20Valid
      (Widget|RemovefromParent (Variables|Default|GetDialogue%20Widget_end)))
    (:Is%20Not%20Valid
      (bind _returnvalue (UserInterface|CreateWidget "/Game/Blueprint/DialogueSystem/Trigger_end.Trigger_end_C" (Game|GetPlayerController 0)))
      (bind _output_get (Variables|Default|SetDialogue%20Widget_end _returnvalue))
      (UserInterface|Viewport|AddtoViewport _output_get 0)
      ;[1 1 1] Prob 1 - Cant take Dialogue widget out and edit text
      (Variables|/Game/Blueprint/DialogueSystem/Trigger_end.Trigger_end_C|SetdialogueEndText (Variables|Default|GetDialogue%20Widget_end) (Variables|Default|GetTriggerText)))))

(fn ConstructionScript)