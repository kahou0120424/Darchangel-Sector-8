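; Story dialogue trigger actor that starts a one-time conversation when the demonicForm_bp player overlaps its StoryCollision.
; On overlap it disables player input, shows a story message widget, hides the interact indicator and plays a timeline that changes the follow camera FOV.
; ExitConversation restores input, reverses the zoom, plays the border disappear animation and removes the widget after a delay.
; Tick re-queries StoryProgress_Msg widgets every frame for that animation.
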(event OnComponentBeginOverlap(storyCollision)
  (params (OverlappedComponent :type Primitive%20Component%20Object%20Reference) (OtherActor :type Actor%20Object%20Reference) (OtherComp :type Primitive%20Component%20Object%20Reference) (OtherBodyIndex :type Integer) (bFromSweep :type Boolean) (SweepResult :type Hit%20Result%20Structure%20%28by%20ref%29))
  (bind _returnvalue (Game|GetPlayerCharacter 0))
  (Utilities|Casting|CastTodemonicForm_bp OtherActor)
  (Utilities|FlowControl|DoOnce false
    (:Completed
      (Variables|Default|SeteisPressed true)
      (Utilities|FlowControl|Sequence
        (:then_0
          (bind _asdemonic_form_bp (Utilities|Casting|CastTodemonicForm_bp _returnvalue))
          (Input|DisableInput _asdemonic_form_bp 0)
          (bind _returnvalue_2 (UserInterface|CreateWidget "/Game/Blueprint/DialogueSystem/StoryProgress_Msg.StoryProgress_Msg_C"))
          (UserInterface|Viewport|AddtoViewport _returnvalue_2 0)
          (Variables|Default|SetisActivated true)
          (Rendering|SetVisibility (Variables|/Game/Blueprint/demonicForm_bp.demonicForm_bp_C|GetInteractIndicator _asdemonic_form_bp) false false))
        (:then_1
          (bind _asdemonic_form_bp_2 (Utilities|Casting|CastTodemonicForm_bp _returnvalue))
          (bind _newtrack_1 (Timeline|StoryZoom Play)
            (:Update
              (Camera|SetFieldOfView (Variables|/Script/Darchangel.MainCharacter|GetFollowCamera _asdemonic_form_bp_2) _newtrack_1))))))))

(event Custom|ExitConversation
  (Variables|Default|SeteisPressed false)
  (Utilities|FlowControl|Sequence
    (:then_0
      (bind _asdemonic_form_bp (Utilities|Casting|CastTodemonicForm_bp (Game|GetPlayerCharacter 0)))
      (Input|EnableInput _asdemonic_form_bp 0)
      (if (Variables|Default|GetisActivated)
        (Utilities|FlowControl|Delay 1.0)
        (Widget|RemovefromParent (stale OnComponentBeginOverlap(storyCollision) _returnvalue_2))))
    (:then_1
      (Utilities|FlowControl|Delay 0.3)
      (bind _newtrack_1 (Timeline|StoryZoom Reverse)
        (:Update
          (Camera|SetFieldOfView (Variables|/Script/Darchangel.MainCharacter|GetFollowCamera (stale OnComponentBeginOverlap(storyCollision) _asdemonic_form_bp_2)) _newtrack_1))))
    (:then_2
      (bind _asstory_progress_msg (Utilities|Casting|CastToStoryProgress_Msg (Utilities|Array|Get(acopy) (stale EventTick _foundwidgets))))
      (UserInterface|Animation|PlayAnimation _asstory_progress_msg (Variables|/Game/Blueprint/DialogueSystem/StoryProgress_Msg.StoryProgress_Msg_C|GetborderDissapearAnimation _asstory_progress_msg) 0.0 1 "Forward" 1.0 false))))

(event Collision|EventActorBeginOverlap
  (params (OtherActor :type Actor%20Object%20Reference)))

(event EventTick
  (params (DeltaSeconds :type Float%20%28single-precision%29))
  (bind _foundwidgets (Widget|GetAllWidgetsOfClass "/Game/Blueprint/DialogueSystem/StoryProgress_Msg.StoryProgress_Msg_C" true)))

(fn ConstructionScript)