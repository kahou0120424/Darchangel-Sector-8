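; Key pickup actor that the demonicForm_bp character collects by touching it.
; On overlap with its Collision component, it increments that character's NumberofKeys, then a DoOnce gate shows the Keyfound_ui widget and plays two pickup sounds at the player before destroying the key.
; The key count increment sits before the DoOnce, so only the feedback and destruction are gated.
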(event OnComponentBeginOverlap(collision)
  (params (OverlappedComponent :type Primitive%20Component%20Object%20Reference) (OtherActor :type Actor%20Object%20Reference) (OtherComp :type Primitive%20Component%20Object%20Reference) (OtherBodyIndex :type Integer) (bFromSweep :type Boolean) (SweepResult :type Hit%20Result%20Structure%20%28by%20ref%29))
  (bind _returnvalue (Game|GetPlayerCharacter 0))
  (bind _returnvalue_2 (Transformation|GetActorLocation _returnvalue))
  (bind _asdemonic_form_bp (Utilities|Casting|CastTodemonicForm_bp OtherActor))
  (Variables|/Game/Blueprint/demonicForm_bp.demonicForm_bp_C|SetnumberofKeys _asdemonic_form_bp (+ (Variables|/Game/Blueprint/demonicForm_bp.demonicForm_bp_C|GetnumberofKeys _asdemonic_form_bp) 1))
  (Utilities|FlowControl|DoOnce false
    (:Completed
      (bind _returnvalue_3 (UserInterface|CreateWidget "/Game/UI/keyUI/keyfound_ui.keyfound_ui_C" (Game|GetPlayerController 0)))
      (UserInterface|Viewport|AddtoViewport _returnvalue_3 0)
      (Audio|PlaySoundatLocation "/Game/Audio/FinalAudio/UI/key/keypickup.keypickup" _returnvalue_2 "0, 0, 0" 1.0 1.0 0.0 0 0 0)
      (Audio|PlaySoundatLocation "/Game/Audio/FinalAudio/UI/key/pickupupdrop.pickupupdrop" _returnvalue_2 "0, 0, 0" 1.0 1.0 0.0 0 0 0)
      (Actor|DestroyActor))))

(event EventBeginPlay)

(event Collision|EventActorBeginOverlap
  (params (OtherActor :type Actor%20Object%20Reference)))

(event EventTick
  (params (DeltaSeconds :type Float%20%28single-precision%29)))

(fn ConstructionScript)