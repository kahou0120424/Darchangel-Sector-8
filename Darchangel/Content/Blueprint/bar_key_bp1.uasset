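; Key-gated barred gate Blueprint that opens for a demonicForm_bp holding enough keys.
; Entering DoorCollision compares NumberofKeys to RequiredKeys, then plays the Gateup timeline to move the mesh's relative location.
; A DoOnce on the timeline update plays a chain-pull sound only once.
; Key deduction is left unconnected, so keys are not consumed; leaving the collision only runs a delay, so nothing closes the gate.
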(event OnComponentBeginOverlap(DoorCollision)
  (params (OverlappedComponent :type Primitive%20Component%20Object%20Reference) (OtherActor :type Actor%20Object%20Reference) (OtherComp :type Primitive%20Component%20Object%20Reference) (OtherBodyIndex :type Integer) (bFromSweep :type Boolean) (SweepResult :type Hit%20Result%20Structure%20%28by%20ref%29))
  (bind _asdemonic_form_bp (Utilities|Casting|CastTodemonicForm_bp OtherActor))
  (if (>= (Variables|/Game/Blueprint/demonicForm_bp.demonicForm_bp_C|GetnumberofKeys _asdemonic_form_bp) (Variables|Default|GetrequiredKeys))
    (bind _newtrack_1 (Timeline|gateup Play)
      (:Update
        (Transformation|SetRelativeLocation (Variables|Default|GetStaticMesh) _newtrack_1 false false)
        (Utilities|FlowControl|DoOnce false
          (:Completed
            (Audio|PlaySound2D "/Game/Audio/chainpul2.chainpul2" 1.0 1.0 0.0 0 0)))))))

(event OnComponentEndOverlap(DoorCollision)
  (params (OverlappedComponent :type Primitive%20Component%20Object%20Reference) (OtherActor :type Actor%20Object%20Reference) (OtherComp :type Primitive%20Component%20Object%20Reference) (OtherBodyIndex :type Integer))
  (Utilities|Casting|CastTodemonicForm_bp OtherActor)
  (Utilities|FlowControl|Delay 3.0))

(event Collision|EventActorBeginOverlap
  (params (OtherActor :type Actor%20Object%20Reference)))

(event EventTick
  (params (DeltaSeconds :type Float%20%28single-precision%29)))

(fn ConstructionScript)