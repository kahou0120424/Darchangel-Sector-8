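; DynamicCamera is a trigger-zone camera actor that takes over the view while the demonicForm_bp character is inside its Start component.
; On overlap it blends player 0's view target to itself over Blendtime and briefly disables that controller's input during the switch.
; When the character leaves, the view blends back to it over the same Blendtime.
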(event OnComponentBeginOverlap(start)
  (params (OverlappedComponent :type Primitive%20Component%20Object%20Reference) (OtherActor :type Actor%20Object%20Reference) (OtherComp :type Primitive%20Component%20Object%20Reference) (OtherBodyIndex :type Integer) (bFromSweep :type Boolean) (SweepResult :type Hit%20Result%20Structure%20%28by%20ref%29))
  (bind _returnvalue (Game|GetPlayerController 0))
  (Utilities|Casting|CastTodemonicForm_bp OtherActor)
  (Game|Player|SetViewTargetwithBlend _returnvalue self (Variables|Default|Getblendtime) "VTBlend_Linear" 0.0 false)
  (Input|DisableInput _returnvalue 0)
  (Utilities|FlowControl|Delay 0.2)
  (Input|EnableInput _returnvalue 0))

(event OnComponentEndOverlap(start)
  (params (OverlappedComponent :type Primitive%20Component%20Object%20Reference) (OtherActor :type Actor%20Object%20Reference) (OtherComp :type Primitive%20Component%20Object%20Reference) (OtherBodyIndex :type Integer))
  (bind _asdemonic_form_bp (Utilities|Casting|CastTodemonicForm_bp OtherActor))
  (Game|Player|SetViewTargetwithBlend (Game|GetPlayerController 0) _asdemonic_form_bp (Variables|Default|Getblendtime) "VTBlend_Linear" 0.0 false))

(event EventBeginPlay)

(event Collision|EventActorBeginOverlap
  (params (OtherActor :type Actor%20Object%20Reference)))

(event EventTick
  (params (DeltaSeconds :type Float%20%28single-precision%29)))

(fn ConstructionScript)