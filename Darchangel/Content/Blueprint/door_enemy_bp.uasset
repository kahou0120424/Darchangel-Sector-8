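; Door actor, named as an enemy door, that swings its right door open when its GateOpen event is called.
; GateOpen plays the DoorOpened timeline, whose Alpha lerps the relative rotation of RightDoor toward the NewLocation rotator.
; Nothing in this file calls GateOpen, and the nodes comparing the count of Ch_Enemy actors with NpcArray are disconnected and never run.
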(event Custom|GateOpen
  (bind _alpha (Timeline|DoorOpened Play)
    (:Update
      (Transformation|SetRelativeRotation (Variables|Default|GetRightDoor) (Math|Rotator|Lerp(Rotator) "0, 0, 0" (Variables|Default|GetnewLocation) _alpha) false false))))

(event Collision|EventActorBeginOverlap
  (params (OtherActor :type Actor%20Object%20Reference)))

(event EventTick
  (params (DeltaSeconds :type Float%20%28single-precision%29)))

(event EventBeginPlay)

(fn ConstructionScript)