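; Test Blueprint for a destructible object that breaks apart under repeated hits from the demonic form character.
; Hits from demonicForm_bp raise a counter until its threshold is met, then enable physics and apply radial damage at the impact point, credited to the demon sword.
; After short delays, it adds a particle effect, switches collision to physics-only and destroys itself.
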(event OnComponentHit(Destructible)
  (params (HitComponent :type Primitive%20Component%20Object%20Reference) (OtherActor :type Actor%20Object%20Reference) (OtherComp :type Primitive%20Component%20Object%20Reference) (NormalImpulse :type Vector :default "0, 0, 0") (Hit :type Hit%20Result%20Structure%20%28by%20ref%29))
  (bind _asdemonic_form_bp (Utilities|Casting|CastTodemonicForm_bp OtherActor))
  (if (>= (Variables|Default|GetisStackedx5?) 1.0)
    (Physics|SetSimulatePhysics (Variables|Default|GetDestructible) true)
    (Game|Damage|ApplyRadialDamage 1e+01 (.ImpactPoint (Collision|BreakHitResult Hit)) 25.0 "/Script/Engine.DamageType" 0 (Variables|/Script/Engine.ChildActorComponent|GetChildActor (Variables|/Game/Blueprint/demonicForm_bp.demonicForm_bp_C|GetWP_Demon_Sword _asdemonic_form_bp)) 0 false "ECC_Visibility")
    (Utilities|FlowControl|Delay 0.5)
    (AddComponent|AddParticleSystemComponent false)
    (Collision|SetCollisionEnabled (Variables|Default|GetDestructible) "PhysicsOnly")
    (Utilities|FlowControl|Delay 5.0)
    (Actor|DestroyActor)
    (else
      (Variables|Default|SetisStackedx5? (+ (Variables|Default|GetisStackedx5?) 1.0)))))

(event EventBeginPlay)

(event Collision|EventActorBeginOverlap
  (params (OtherActor :type Actor%20Object%20Reference)))

(event EventTick
  (params (DeltaSeconds :type Float%20%28single-precision%29)))

(fn ConstructionScript)