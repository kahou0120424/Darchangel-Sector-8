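; Enemy wave spawner actor that creates NPC_BP_1 AI running NPC_BT at random points inside the SpawnArea bounds.
; When demonicForm_bp overlaps SpawnTrigger, the EnemyWaves timeline fires Wave 1 spawns and sets Wave1Done.
; Tick polls that flag, which is never reset here, then delays, re-checks the overlapping actor's class and plays a second timeline for Wave 2 spawns.
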(event OnComponentBeginOverlap(SpawnTrigger)
  (params (OverlappedComponent :type Primitive%20Component%20Object%20Reference) (OtherActor :type Actor%20Object%20Reference) (OtherComp :type Primitive%20Component%20Object%20Reference) (OtherBodyIndex :type Integer) (bFromSweep :type Boolean) (SweepResult :type Hit%20Result%20Structure%20%28by%20ref%29))
  (bind _spawnarea (Variables|Default|GetSpawnArea))
  (bind _boxextent (Collision|GetComponentBounds _spawnarea))
  (Utilities|FlowControl|Sequence
    (:then_0
      (Utilities|Casting|CastTodemonicForm_bp OtherActor)
      (Timeline|EnemyWaves Play
        (:Wave%201
          (AI|SpawnAIFromClass "/Game/AI/NPC_BP_1.NPC_BP_1_C" "/Game/AI/NPC_BT.NPC_BT" (+ (Math|Vector|MakeVector (Math|Random|RandomFloatinRange (* (.x _boxextent) -1.0) (.x _boxextent)) (Math|Random|RandomFloatinRange (* (.y _boxextent) -1.0) (.y _boxextent)) (Math|Random|RandomFloatinRange (* (.z _boxextent) -1.0) (.z _boxextent))) (Transformation|GetWorldLocation _spawnarea)) "0, 0, 0" false)
          (Variables|Default|Setwave1Done true))))))

(event EventBeginPlay)

(event Collision|EventActorBeginOverlap
  (params (OtherActor :type Actor%20Object%20Reference)))

(event EventTick
  (params (DeltaSeconds :type Float%20%28single-precision%29))
  (bind _spawnarea (Variables|Default|GetSpawnArea))
  (bind _boxextent (Collision|GetComponentBounds _spawnarea))
  (if (Variables|Default|Getwave1Done)
    (Utilities|FlowControl|Delay 5.0)
    (Utilities|Casting|CastTodemonicForm_bp (stale OnComponentBeginOverlap(SpawnTrigger) OtherActor))
    (Timeline|Timeline_0 Play
      (:Wave%202
        (AI|SpawnAIFromClass "/Game/AI/NPC_BP_1.NPC_BP_1_C" "/Game/AI/NPC_BT.NPC_BT" (+ (Math|Vector|MakeVector (Math|Random|RandomFloatinRange (* (.x _boxextent) -1.0) (.x _boxextent)) (Math|Random|RandomFloatinRange (* (.y _boxextent) -1.0) (.y _boxextent)) (Math|Random|RandomFloatinRange (* (.z _boxextent) -1.0) (.z _boxextent))) (Transformation|GetWorldLocation _spawnarea)) "0, 0, 0" false)))))

(fn ConstructionScript)