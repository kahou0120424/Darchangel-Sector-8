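; Enemy spawner actor that places AI-controlled Ch_Enemy pawns at random points inside its Box component.
; On Tick, while fewer than 10 NPC_BP_1 actors exist, a retriggerless Delay throttles spawning to roughly every five seconds, with each pawn running NPC_BT.
; The limit counts a different class from the one spawned.
; An unconnected variant that counts Ch_Enemy with a shorter delay and no behavior tree never runs.
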(event EventBeginPlay)

(event Collision|EventActorBeginOverlap
  (params (OtherActor :type Actor%20Object%20Reference)))

(event EventTick
  (params (DeltaSeconds :type Float%20%28single-precision%29))
  (bind _box (Variables|Default|GetBox))
  (bind _outactors (Actor|GetAllActorsOfClass "/Game/AI/NPC_BP_1.NPC_BP_1_C"))
  (if (< (Utilities|Array|Length _outactors) 10)
    (Utilities|FlowControl|Delay 5.0)
    (AI|SpawnAIFromClass "/Game/AI/Ch_Enemy.Ch_Enemy_C" "/Game/AI/NPC_BT.NPC_BT" (Math|Random|RandomPointinBoundingBox (Transformation|GetWorldLocation _box) (Components|Box|GetScaledBoxExtent _box)) "0, 0, 0" false)))

(fn ConstructionScript)