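; Key-locked double door Actor that opens when the demonicForm_bp player character enters its DoorCollision volume with enough keys.
; On overlap it subtracts RequiredKeys from the player's NumberofKeys, then plays two timelines that lerp the right and left door rotations to their target rotators.
; End overlap only runs a three-second delay with nothing after it, so the doors never close.
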(event OnComponentBeginOverlap(DoorCollision)
  (params (OverlappedComponent :type Primitive%20Component%20Object%20Reference) (OtherActor :type Actor%20Object%20Reference) (OtherComp :type Primitive%20Component%20Object%20Reference) (OtherBodyIndex :type Integer) (bFromSweep :type Boolean) (SweepResult :type Hit%20Result%20Structure%20%28by%20ref%29))
  (bind _requiredkeys (Variables|Default|GetrequiredKeys))
  (bind _asdemonic_form_bp (Utilities|Casting|CastTodemonicForm_bp OtherActor))
  (if (>= (Variables|/Game/Blueprint/demonicForm_bp.demonicForm_bp_C|GetnumberofKeys _asdemonic_form_bp) _requiredkeys)
    (Variables|/Game/Blueprint/demonicForm_bp.demonicForm_bp_C|SetnumberofKeys _asdemonic_form_bp (- (Variables|/Game/Blueprint/demonicForm_bp.demonicForm_bp_C|GetnumberofKeys _asdemonic_form_bp) _requiredkeys))
    (Utilities|FlowControl|Sequence
      (:then_0
        (bind _alpha (Timeline|RightDoorMovement Play)
          (:Update
            (Transformation|SetRelativeRotation (Variables|Default|GetRightDoor) (Math|Rotator|Lerp(Rotator) "0, 0, 0" (Variables|Default|GetrightLocation) _alpha) false false))))
      (:then_1
        (bind _alpha_2 (Timeline|LeftDoorMovement Play)
          (:Update
            (Transformation|SetRelativeRotation (Variables|Default|GetLeftDoor) (Math|Rotator|Lerp(Rotator) "0, 0, 0" (Variables|Default|GetleftLocation) _alpha_2) false false)))))))

(event OnComponentEndOverlap(DoorCollision)
  (params (OverlappedComponent :type Primitive%20Component%20Object%20Reference) (OtherActor :type Actor%20Object%20Reference) (OtherComp :type Primitive%20Component%20Object%20Reference) (OtherBodyIndex :type Integer))
  (Utilities|Casting|CastTodemonicForm_bp OtherActor)
  (Utilities|FlowControl|Delay 3.0))

(event EventBeginPlay)

(event Collision|EventActorBeginOverlap
  (params (OtherActor :type Actor%20Object%20Reference)))

(event EventTick
  (params (DeltaSeconds :type Float%20%28single-precision%29)))

(fn ConstructionScript)