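; Hideable wall arch that fades its static mesh out and back in when told to hide or show.
; BeginPlay creates a dynamic material instance from the mesh's first material.
; The Show and Hide functions set opposing flags that Tick polls, passing delta time scaled by FadeSpeed to UpdateVisibility.
; UpdateVisibility steps the Opacity parameter and clears the active flag once it reaches fully transparent or fully opaque.
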(event EventBeginPlay
  (bind _staticmesh (Variables|Default|GetStaticMesh))
  (bind _returnvalue (Rendering|Material|CreateDynamicMaterialInstance _staticmesh 0 (Rendering|Material|GetMaterial _staticmesh 0) "None" :!class /Script/Engine.PrimitiveComponent))
  (Variables|Default|SetDynamicMaterial _returnvalue))

(event EventTick
  (params (DeltaSeconds :type Float%20%28single-precision%29))
  (bind _hide_ (Variables|Default|GetHide?))
  (if _hide_
    (CallFunction|UpdateVisibility (* DeltaSeconds (Variables|Default|GetFadeSpeed)) _hide_ :!label _label)
    (elif (Variables|Default|GetShow?)
      (goto _label))))

(fn ConstructionScript)

(fn UpdateVisibility
  (params (Amount :type Float%20%28single-precision%29) (Hide? :type Boolean))
  (bind _dynamicmaterial (Variables|Default|GetDynamicMaterial))
  (bind _returnvalue (Rendering|Material|GetScalarParameterValue _dynamicmaterial "Opacity" :!class /Script/Engine.MaterialInstanceDynamic))
  (if Hide?
    (Rendering|Material|SetScalarParameterValue _dynamicmaterial "Opacity" (- _returnvalue Amount) :!class /Script/Engine.MaterialInstanceDynamic)
    (Variables|Default|SetHide? (not (<= (- _returnvalue Amount) 0.0)))
    (else
      (Rendering|Material|SetScalarParameterValue _dynamicmaterial "Opacity" (+ _returnvalue Amount) :!class /Script/Engine.MaterialInstanceDynamic)
      (Variables|Default|SetShow? (not (>= (+ _returnvalue Amount) 1.0)))))
  (return))

(fn Show
  (Variables|Default|SetShow? true)
  (Variables|Default|SetHide? false)
  (return))

(fn Hide
  (Variables|Default|SetShow? false)
  (Variables|Default|SetHide? true)
  (return))